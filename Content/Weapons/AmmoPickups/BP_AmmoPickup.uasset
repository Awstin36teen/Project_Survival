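; Ammo pickup actor that tops up one caliber on a BP_PlayerPawn overlapping it while below max ammo, then destroys itself.
; A switch on AmmoCaliber calls a per-caliber macro that adds to the matching count before the player's UpdateAmmoCount runs.
; The random amount rolled at BeginPlay is unused, as macros add AmmoCountMax.
; The 30 Carbine macro writes its result into 300BLKCount.
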(event Collision|EventActorBeginOverlap
  (params (OtherActor :type Actor%20Object%20Reference))
  (bind _asbp_player_pawn (Utilities|Casting|CastToBP_PlayerPawn OtherActor))
  ;[1 1 1] Player Has Room for more ammo
  (if (< (Variables|/Game/PlayerChar/Player/BP_PlayerPawn.BP_PlayerPawn_C|GetCurrent_Ammo_Count _asbp_player_pawn) (Variables|/Game/PlayerChar/Player/BP_PlayerPawn.BP_PlayerPawn_C|GetMax_Ammo_Count _asbp_player_pawn))
    ;[1 1 1] Give Player Ammo
    (Variables|Default|SetTarget%20PLayer _asbp_player_pawn)
    (switch Utilities|FlowControl|Switch|SwitchonE_Caliber (Variables|Default|GetAmmo%20%20caliber)
      (:NewEnumerator0
        (|22lr))
      (:NewEnumerator1
        (|20carbine))
      (:NewEnumerator2
        (|25acp))
      (:NewEnumerator3
        (|300BLK))
      (:NewEnumerator4
        (|380acp))
      (:NewEnumerator5
        (|56x45mm))
      (:NewEnumerator6
        (|9mm))
      (:NewEnumerator7
        (|40s&w))
      (:NewEnumerator8
        (|62x51))
      (:NewEnumerator9
        (|45acp))
      (:NewEnumerator10
        (|10mm))
      (:NewEnumerator12
        (|357magnum))
      (:NewEnumerator17
        (|50Cal))
      (:NewEnumerator14
        (|BirdShot))
      (:NewEnumerator15
        (|BuckShot))
      (:NewEnumerator16
        (|Slugs)))
    ;[1 1 1] Update Current Ammo (Player)
    (Default|UpdateAmmoCount (Variables|Default|GetTarget%20PLayer))
    ;[1 1 1] Remove Self Form Enviment
    (Actor|DestroyActor)))

(event EventBeginPlay
  (Variables|Default|SetAmmo%20Count_%20Current (Math|Random|RandomFloatinRange (Variables|Default|GetAmmo%20Count_%20Min) (Variables|Default|GetAmmo%20Count_%20Max))))

(fn ConstructionScript)