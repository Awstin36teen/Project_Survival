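; BP_TracerMaster is the base weapon tracer actor that flies toward a TargetLocation and destroys itself on arrival.
; Each Tick it snaps its rotation to face the target and moves along local X at MoveSpeed without sweeping, until it is within a small tolerance of that point.
; A lifespan set on BeginPlay acts as a fallback cleanup.
; An interpolated-rotation node is left unconnected, so turning is instant.
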(event EventBeginPlay
  (Actor|SetLifeSpan 1.2e+02))

(event EventTick
  (params (DeltaSeconds :type Float%20%28single-precision%29))
  (if (Math|Vector|NotEqual(Vector) (Variables|Default|GetTargetLocation) (Transformation|GetActorLocation) 25.0)
    (Transformation|SetActorRotation (Math|Rotator|FindLookatRotation (Transformation|GetActorLocation) (Variables|Default|GetTargetLocation)))
    (Transformation|AddActorLocalOffset (Math|Vector|MakeVector (* (Utilities|Time|GetWorldDeltaSeconds) (Variables|Default|GetMove%20Speed)) 0.0 0.0) false false)
    (else
      (Actor|DestroyActor))))

(fn ConstructionScript)